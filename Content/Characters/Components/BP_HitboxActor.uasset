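; Fighting-game hitbox actor that serves as a proximity box, strike box or hurtbox according to its HitboxType.
; SpawnHitbox applies a type-specific material to the display component, moves it to HitboxLocation and makes it visible.
; On overlap, only the strike type acts, inflicting fixed damage on any AFighterBase other than its OwningPlayer.
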(event `self.ReceiveActorBeginOverlap`
  (params (OtherActor :type "Actor Object Reference"))
  (if (`|EnumEquality` (`self.HitboxType`) "HB_STRIKE")
    (bind _asafighter_base (cast `AFighterBase` OtherActor))
    (if (!= _asafighter_base (`self.OwningPlayer`))
      (`AFighterBase.InflictDamage` _asafighter_base 1000))))

(event `Spawn Hitbox`
  (switch `EHitboxEnum` (`self.HitboxType`)
    (:`HB_PROXIMITY`
      (`PrimitiveComponent.SetMaterial` (`self.Hitbox Display`) 0 "/Engine/MapTemplates/Materials/BasicAsset02.BasicAsset02"))
    (:`HB_STRIKE`
      (`PrimitiveComponent.SetMaterial` (`self.Hitbox Display`) 0 "/Engine/MapTemplates/Materials/BasicAsset03.BasicAsset03"))
    (:`HB_HURTBOX`
      (`PrimitiveComponent.SetMaterial` (`self.Hitbox Display`) 0 "/Engine/BasicShapes/BasicShapeMaterial.BasicShapeMaterial")))
  (`SceneComponent.K2_SetWorldLocation` (`self.Hitbox Display`) (`self.HitboxLocation`) false false)
  (`SceneComponent.SetVisibility` (`self.Hitbox Display`) true false))

(fn `UserConstructionScript`)